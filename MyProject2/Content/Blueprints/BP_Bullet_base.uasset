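; BP_Bullet_base is a bullet actor, apparently a base class, that flies forward from the moment it spawns.
; A self-calling Move event advances the Sphere component along its forward vector by MoveSpeed with sweep, repeating after a short Delay instead of using Tick or a projectile movement component.
; The Hit event only checks whether the other actor differs from the player pawn, with no damage or destroy logic attached.
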(event Custom|Move
  (bind _sphere (Variables|Default|GetSphere))
  (Transformation|SetWorldLocation _sphere (+ (Transformation|GetWorldLocation _sphere) (* (Math|Vector|GetForwardVector _sphere) (Variables|Default|GetMove%20Speed))) true false)
  (Utilities|FlowControl|Delay 0.01)
  (CallFunction|Move))

(event EventBeginPlay
  (CallFunction|Move))

(event Collision|EventHit
  (params (MyComp :type Primitive%20Component%20Object%20Reference) (Other :type Actor%20Object%20Reference) (OtherComp :type Primitive%20Component%20Object%20Reference) (bSelfMoved :type Boolean) (HitLocation :type Vector :default "0, 0, 0") (HitNormal :type Vector :default "0, 0, 0") (NormalImpulse :type Vector :default "0, 0, 0") (Hit :type Hit%20Result%20Structure%20%28by%20ref%29))
  (if (!= Other (Game|Player|GetPlayerPawn 0))
    _))

(fn ConstructionScript)