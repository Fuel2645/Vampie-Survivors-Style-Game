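; BP_enemy is an AI enemy pawn that chases the player and shows a health bar widget.
; A recursive delay loop yaws its Cube toward the player, while Move repeatedly issues short AIMoveTo steps along the Cube's forward vector, re-arming only on success.
; Damage clamps health, updates the bar and destroys the actor at zero.
; Poison hits immediately, then repeats through a looping timer until ended, ignoring new starts while active.
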(event Custom|Move
  (bind _cube (Variables|Default|GetCube))
  (AI|AIMoveTo self (+ (Transformation|GetWorldLocation _cube) (* (Math|Vector|GetForwardVector _cube) 5.0)) 0 1.0 false
    (:OnSuccess
      (CallFunction|Move))))

(event Custom|Rotation
  (Transformation|SetWorldRotation (Variables|Default|GetCube) (Math|Rotator|MakeRotator 0.0 0.0 (.yaw (Math|Rotator|FindLookatRotation (Transformation|GetWorldLocation (Variables|Default|GetCube)) (Transformation|GetActorLocation (Game|Player|GetPlayerPawn 0))))) false false)
  (Utilities|FlowControl|Delay 0.1)
  (CallFunction|Rotation))

(event Custom|PoisonDamage
  (CallFunction|Damage (Variables|Poison|Getpoison%20Damage)))

(event EventPoisonDamageStart
  (params (inDamage :type Float%20%28single-precision%29) (TimeBetween :type Float%20%28single-precision%29))
  (if (not (Utilities|Time|IsTimerActivebyHandle (Variables|Poison|GetPoisonTimer)))
    (CallFunction|Damage inDamage)
    (bind _returnvalue (Utilities|Time|SetTimerbyEvent (delegate Custom|PoisonDamage) TimeBetween true))
    (Variables|Poison|SetPoisonTimer _returnvalue)
    (Variables|Poison|Setpoison%20Damage inDamage)))

(event EventBeginPlay
  (CallFunction|Rotation)
  (CallFunction|Move)
  (bind _aswbp_enemy_hpbar (Utilities|Casting|CastToWBP_EnemyHPBar (UserInterface|GetWidget (Variables|Default|GetWidget))))
  (Progress|SetPercent (Variables|/Game/Blueprints/Widgets/WBP_EnemyHPBar.WBP_EnemyHPBar_C|GetProgressBar_0 _aswbp_enemy_hpbar) (/ (Variables|Default|GetHealth) (Variables|Default|GetMax%20Health))))

(event EventPoisonDamageEnd
  (bind _poisontimer (Variables|Poison|GetPoisonTimer))
  (Utilities|Time|PauseTimerbyHandle _poisontimer)
  (Utilities|Time|ClearandInvalidateTimerbyHandle _poisontimer))

(event EventDamage
  (params (inDamage :type Float%20%28single-precision%29))
  (bind _output_get (Variables|Default|SetHealth (Math|Float|Clamp(Float) (- (Variables|Default|GetHealth) inDamage) 0.0 (Variables|Default|GetMax%20Health))))
  (if (== _output_get 0.0)
    (Actor|DestroyActor)
    (else
      (bind _aswbp_enemy_hpbar (Utilities|Casting|CastToWBP_EnemyHPBar (UserInterface|GetWidget (Variables|Default|GetWidget))))
      (Progress|SetPercent (Variables|/Game/Blueprints/Widgets/WBP_EnemyHPBar.WBP_EnemyHPBar_C|GetProgressBar_0 _aswbp_enemy_hpbar) (/ (Variables|Default|GetHealth) (Variables|Default|GetMax%20Health))))))

(fn ConstructionScript)