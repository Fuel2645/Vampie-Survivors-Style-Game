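; Player character Blueprint that handles Enhanced Input movement, cursor aiming, shooting, dashing and three abilities.
; Mouse2D yaws the Cube toward the cursor hit, while shooting spawns rebounding bullets from the Gun behind a DoOnce/Delay cooldown.
; Abilities activate timer-gated rotating balls and cleave components or spawn a yaw-offset boomerang.
; Dash launches along the last movement vector, briefly slowing global time while compensating the player's own dilation.
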(event Input|EnhancedActionEvents|EnhancedInputActionIA_Movement
  (params (ActionValue :type Vector%202D%20Structure) (ElapsedSeconds :type Float%20%28double-precision%29) (TriggeredSeconds :type Float%20%28double-precision%29) (InputAction :type Input%20Action%20Object%20Reference :default "/Game/Input/IA_Movement.IA_Movement"))
  (bind (_x _y) (Math|Vector2D|BreakVector2D ActionValue))
  (bind _mesh (Variables|Character|GetMesh))
  (bind _output_get (Variables|Default|Setm_MovementVector (+ (* _x (Math|Vector|GetForwardVector _mesh)) (* _y (Math|Vector|GetRightVector _mesh)))))
  (Pawn|Input|AddMovementInput _output_get 1.0 false))

(event Input|EnhancedActionEvents|EnhancedInputActionIA_Shoot
  (params (ActionValue :type Boolean) (ElapsedSeconds :type Float%20%28double-precision%29) (TriggeredSeconds :type Float%20%28double-precision%29) (InputAction :type Input%20Action%20Object%20Reference :default "/Game/Input/IA_Shoot.IA_Shoot"))
  (bind _gun (Variables|Default|GetGun))
  (bind _returnvalue (Transformation|GetWorldTransform _gun))
  (bind (_location _rotation) (Math|Transform|BreakTransform _returnvalue))
  (Utilities|FlowControl|DoOnce false :!label _label
    (:Completed
      (Game|SpawnActorfromClass "/Script/MyProject2.Bullet_Rebound" (Math|Transform|MakeTransform (+ _location (* (Math|Vector|GetForwardVector _gun) 1e+01)) _rotation "1.000000,1.000000,1.000000") "AlwaysSpawn" "MultiplyWithRoot" 0 0)
      (Utilities|FlowControl|Delay 0.2)
      (goto _label Reset))))

(event Input|EnhancedActionEvents|EnhancedInputActionIA_Ability1
  (params (ActionValue :type Boolean) (ElapsedSeconds :type Float%20%28double-precision%29) (TriggeredSeconds :type Float%20%28double-precision%29) (InputAction :type Input%20Action%20Object%20Reference :default "/Game/Input/IA_Ability1.IA_Ability1"))
  (:Started
    (if (not (Utilities|Time|IsTimerActivebyHandle (Variables|/Script/MyProject2.BaseAbilityComponent|GetDurationTimer (Variables|Default|GetRotatingBallsAbility))))
      (Class|BaseAbilityComponent|Activation (Variables|Default|GetRotatingBallsAbility)))))

(event Input|EnhancedActionEvents|EnhancedInputActionIA_Ability2
  (params (ActionValue :type Boolean) (ElapsedSeconds :type Float%20%28double-precision%29) (TriggeredSeconds :type Float%20%28double-precision%29) (InputAction :type Input%20Action%20Object%20Reference :default "/Game/Input/IA_Ability2.IA_Ability2"))
  (:Started
    (Class|BaseAbilityComponent|Activation (Variables|Default|GetCleaveAbility))))

(event Input|EnhancedActionEvents|EnhancedInputActionIA_Ability3
  (params (ActionValue :type Boolean) (ElapsedSeconds :type Float%20%28double-precision%29) (TriggeredSeconds :type Float%20%28double-precision%29) (InputAction :type Input%20Action%20Object%20Reference :default "/Game/Input/IA_Ability3.IA_Ability3"))
  (bind _gun (Variables|Default|GetGun))
  (bind _returnvalue (Transformation|GetWorldRotation _gun))
  (:Started
    (Game|SpawnActorfromClass "/Script/MyProject2.Boomerang" (Math|Transform|MakeTransform (Transformation|GetWorldLocation _gun) (Math|Rotator|MakeRotator (.roll _returnvalue) (.pitch _returnvalue) (- (.yaw _returnvalue) 6e+01)) "1.000000,1.000000,1.000000") "Undefined" "MultiplyWithRoot" 0 0)))

(event Input|EnhancedActionEvents|EnhancedInputActionIA_Dash
  (params (ActionValue :type Boolean) (ElapsedSeconds :type Float%20%28double-precision%29) (TriggeredSeconds :type Float%20%28double-precision%29) (InputAction :type Input%20Action%20Object%20Reference :default "/Game/Input/IA_Dash.IA_Dash"))
  (:Started
    (Character|LaunchCharacter (* (Variables|Default|Getm_MovementVector) 1e+03) false false)
    (Utilities|Time|SetGlobalTimeDilation 0.25)
    (Variables|Default|SetCustomTimeDilation 4.0)
    (Utilities|FlowControl|Delay 0.1)
    (Utilities|Time|SetGlobalTimeDilation 1.0)
    (Variables|Default|SetCustomTimeDilation 1.0)))

(event EventBeginPlay
  (Input|AddMappingContext (PlayerController|LocalPlayerSubsystems|GetEnhancedInputLocalPlayerSubsystem (Game|GetPlayerController 0)) "/Game/Input/IMC_PLayer.IMC_PLayer" 0 "(bIgnoreAllPressedKeysUntilRelease=True,bForceImmediately=False,bNotifyUserSettings=False)")
  (Variables|/Script/MyProject2.BaseAbilityComponent|SetAbilityDuration (Variables|Default|GetRotatingBallsAbility) 3.0))

(event Input|MouseEvents|Mouse2D
  (params (AxisValue :type Vector :default "0, 0, 0"))
  (Transformation|SetWorldRotation (Variables|Default|GetCube) (Math|Rotator|MakeRotator 0.0 0.0 (.yaw (Math|Rotator|FindLookatRotation (Transformation|GetWorldLocation (Variables|Default|GetCube)) (.location (.HitResult (Game|Player|GetHitResultUnderCursorbyChannel (Game|GetPlayerController 0) "TraceTypeQuery3" true)))))) false false))

(fn ConstructionScript)